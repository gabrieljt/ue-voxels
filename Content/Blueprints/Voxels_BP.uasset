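; Voxel map Blueprint that builds a solid cubic block of randomly mixed grass and dirt cubes at BeginPlay.
; It creates two instanced static mesh components, one per cube type, to render the voxels as instances.
; Triple nested loops add each instance to a randomly picked component, converting grid indices to positions by scaling with twice a randomly picked mesh's bounding box max.
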(event EventBeginPlay
  ;[1 1 1] Set Static Meshes for Instaced Static Mesh Components
  (bind _returnvalue (AddComponent|AddInstancedStaticMeshComponent false))
  (bind _output_get (Variables|Default|SetInstancedStaticMeshComponent (Utilities|Array|MakeArray _returnvalue (stale _returnvalue_2))))
  (Components|StaticMesh|SetStaticMesh (Utilities|Array|Get(acopy) _output_get) "/Game/StaticMeshes/GrassCube.GrassCube")
  (bind _returnvalue_2 (AddComponent|AddInstancedStaticMeshComponent false))
  (bind _output_get_2 (Variables|Default|SetInstancedStaticMeshComponent (Utilities|Array|MakeArray _returnvalue _returnvalue_2)))
  (Components|StaticMesh|SetStaticMesh (Utilities|Array|Get(acopy) _output_get_2 1) "/Game/StaticMeshes/DirtCube.DirtCube")
  ;[1 1 1] Generate Voxel Map
  (for _index (range 0 9)
    (for _index_2 (range 0 9)
      (for _index_3 (range 0 9)
        ;[1 1 1] Add Selected Static Mesh Instance
        (Components|InstancedStaticMesh|AddInstance (Utilities|Array|Get(acopy) (Variables|Default|GetInstancedStaticMeshComponent) (Math|Random|RandomInteger 2)) (Math|Transform|MakeTransform (* (* (Math|Vector|MakeVector (Math|Conversions|ToFloat(Integer) _index) (Math|Conversions|ToFloat(Integer) _index_2) (Math|Conversions|ToFloat(Integer) _index_3)) 2.0) (.Max (Utilities|Struct|BreakBox (StaticMesh|GetBoundingBox (Variables|/Script/Engine.StaticMeshComponent|GetStaticMesh (Utilities|Array|Get(acopy) (Variables|Default|GetInstancedStaticMeshComponent) (Math|Random|RandomInteger 2)))))))))))))

(fn ConstructionScript)
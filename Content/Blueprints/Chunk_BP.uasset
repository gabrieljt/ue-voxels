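; Voxel chunk actor that fills a cubic grid with randomly chosen grass and dirt cubes on BeginPlay.
; A helper function creates one Instanced Static Mesh component per block type at runtime, each assigned its own cube mesh.
; A triple loop over ChunkSize adds an instance to a random component at each grid cell, spaced by the mesh bounding box.
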(event EventBeginPlay
  (bind _returnvalue (Math|Random|RandomInteger 2))
  (bind _chunk_size (Variables|Default|GetChunk%20Size))
  (bind _instanced_static_mesh_components (Variables|Default|GetInstanced%20Static%20Mesh%20Components))
  (bind _item (Utilities|Array|Get(acopy) _instanced_static_mesh_components _returnvalue))
  (bind _instancedstaticmeshcomponents (CallFunction|SetInstancedStaticMeshComponents 2))
  ;[1 1 1] Set Static Meshes for Instaced Static Mesh Components: one Static Mesh per Material (necessary?)
  (Components|StaticMesh|SetStaticMesh (Utilities|Array|Get(acopy) _instancedstaticmeshcomponents) "/Game/StaticMeshes/GrassCube.GrassCube")
  (Components|StaticMesh|SetStaticMesh (Utilities|Array|Get(acopy) _instancedstaticmeshcomponents 1) "/Game/StaticMeshes/DirtCube.DirtCube")
  ;[1 1 1] Generate Voxel Map
  (for _index (range 0 _chunk_size)
    (for _index_2 (range 0 _chunk_size)
      (for _index_3 (range 0 _chunk_size)
        ;[1 1 1] Add Selected Static Mesh Instance
        (Components|InstancedStaticMesh|AddInstance _item (Math|Transform|MakeTransform (* (* (Math|Vector|MakeVector (Math|Conversions|ToFloat(Integer) _index) (Math|Conversions|ToFloat(Integer) _index_2) (Math|Conversions|ToFloat(Integer) _index_3)) 2.0) (.Max (Utilities|Struct|BreakBox (StaticMesh|GetBoundingBox (Variables|/Script/Engine.StaticMeshComponent|GetStaticMesh _item)))))))))))

(fn ConstructionScript)

(fn SetInstancedStaticMeshComponents
  (params (NumberOfStaticMeshes :type Integer))
  (bind _instanced_static_mesh_components (Variables|Default|GetInstanced%20Static%20Mesh%20Components))
  (for _index (range 0 NumberOfStaticMeshes)
    (bind _returnvalue (AddComponent|AddInstancedStaticMeshComponent false))
    (Utilities|Array|SetArrayElem _instanced_static_mesh_components _index _returnvalue true))
  (return _instanced_static_mesh_components))